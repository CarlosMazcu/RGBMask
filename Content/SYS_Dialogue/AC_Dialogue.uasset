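; Dialogue actor component that shows a sequence of text lines in an on-screen dialogue box.
; StartDialogue uses the component's active state to block re-entry, creates the widget, passes itself to it, gives it keyboard focus in UI-only input and shows the first line.
; AdvanceDialogue steps through the lines array and calls EndDialogue after the last, which removes the widget, deactivates the component and restores game-only input.
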(event EventBeginPlay)

(event EventTick
  (params (DeltaSeconds :type Float%20%28single-precision%29)))

(fn StartDialogue
  (bind _returnvalue (Game|GetPlayerController 0))
  (if (not (Components|Activation|IsActive))
    (Components|Activation|SetActive true false)
    (Variables|Default|SetIndex 0)
    (Utilities|FlowControl|Sequence
      (:then_0
        ;[0.15 0.15 0.15 0.5] Create Widget
        (bind _returnvalue_2 (UserInterface|CreateWidget (Variables|Default|GetDialogueBoxClass) _returnvalue))
        (UserInterface|Viewport|AddtoViewport _returnvalue_2 0)
        (Input|SetInputModeUIOnly _returnvalue _returnvalue_2 "DoNotLock" false)
        (bind _output_get (Variables|Default|SetDialogueBoxWidget _returnvalue_2))
        (Variables|/Game/SYS_Dialogue/WBP_DialogueBox.WBP_DialogueBox_C|SetDialogueComp _output_get self)
        (Widget|SetKeyboardFocus _output_get))
      (:then_1
        ;[0.15 0.15 0.15 0.5] Initialize the Dialogue line
        (Rendering|Components|TextRender|SetText (Variables|/Game/SYS_Dialogue/WBP_DialogueBox.WBP_DialogueBox_C|GetDialogueText (Variables|Default|GetDialogueBoxWidget)) (Utilities|Array|Get(acopy) (Variables|Default|GetDialogueLines)))))))

(fn AdvanceDialogue
  (bind _result (Math|Integer|IncrementInt (Variables|Default|GetIndex))
    (:%20%20
      (if (< _result (Utilities|Array|Length (Variables|Default|GetDialogueLines)))
        (Rendering|Components|TextRender|SetText (Variables|/Game/SYS_Dialogue/WBP_DialogueBox.WBP_DialogueBox_C|GetDialogueText (Variables|Default|GetDialogueBoxWidget)) (Utilities|Array|Get(acopy) (Variables|Default|GetDialogueLines) (Variables|Default|GetIndex)))
        (else
          (CallFunction|EndDialogue))))))

(fn EndDialogue
  (Widget|RemovefromParent (Variables|Default|GetDialogueBoxWidget))
  (Components|Activation|SetActive false false)
  (Input|SetInputModeGameOnly (Game|GetPlayerController 0) false))