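; Pickup actor that the top-down character collects by overlapping it, acting as a mask, key or coin based on its IsMask and IsKey flags.
; An ActorSequence animation loops from BeginPlay.
; Masks add their MaskType to the character's inventory and keys fire the OnKeyPicked dispatcher, then both destroy themselves.
; Otherwise it increments the character's Coins and prints the total, without destroying the actor.
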(event EventBeginPlay
  (Class|MovieSceneSequencePlayer|PlayLooping (Variables|/Script/ActorSequence.ActorSequenceComponent|GetSequencePlayer (Variables|Default|GetActorSequence)) -1))

(event Collision|EventActorBeginOverlap
  (params (OtherActor :type Actor%20Object%20Reference))
  (bind _asbp_top_down_character (Utilities|Casting|CastToBP_TopDownCharacter OtherActor))
  (if (Variables|Mask|GetisMask)
    (Class|RGBMaskCharacter|AddMasktoInventory _asbp_top_down_character (Variables|Mask|GetMaskType))
    (Actor|DestroyActor)
    (elif (Variables|Key|GetisKey)
      (Default|CallOnKeyPicked self)
      (Actor|DestroyActor)
      (else
        ;[0.15 0.15 0.15 0.5] Is NOT a MASK
        (bind _result (Math|Integer|IncrementInt (Variables|/Game/TopDown/Blueprints/BP_TopDownCharacter.BP_TopDownCharacter_C|GetCoins _asbp_top_down_character))
          (:%20%20
            (bind _output_get (Variables|/Game/TopDown/Blueprints/BP_TopDownCharacter.BP_TopDownCharacter_C|SetCoins _asbp_top_down_character _result))
            (Development|PrintString "Coin added")
            (Development|PrintString (Utilities|String|Append (Utilities|String|ToString(Integer) _output_get) " coins"))))))))

(fn ConstructionScript)