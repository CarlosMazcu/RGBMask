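; BP_DoorMechanism is a door actor that opens by disappearing once every pickup in its KeysNeeded list has been collected.
; On BeginPlay it binds to each key's picked event, removing that key from the list when it fires.
; When the list empties, a timed cutscene disables player input, blends the view to the door and hides it.
; It then blends back to the top-down character, destroys itself and restores input.
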(event Custom|EmptyKeysNeeded
  (params (Caller :type Actor%20Object%20Reference))
  (bind _returnvalue (Game|GetPlayerController 0))
  (bind _keysneeded (Variables|Keys|GetKeysNeeded))
  (bind _blend_time (Variables|Default|GetBlend%20Time))
  (bind _waitingtime (Variables|Default|GetWaitingTime))
  (bind _asbp_pickup (Utilities|Casting|CastToBP_Pickup Caller))
  (Utilities|Array|RemoveItem _keysneeded _asbp_pickup)
  (if (Utilities|Array|IsEmpty _keysneeded)
    (Input|DisableInput (Game|Player|GetPlayerPawn 0) _returnvalue)
    (Game|Player|SetViewTargetwithBlend _returnvalue self (Variables|Default|GetBlend%20Time) "VTBlend_Linear" 0.0 false)
    (Utilities|FlowControl|Delay _waitingtime)
    (Rendering|SetActorHiddenInGame true)
    (Utilities|FlowControl|Delay (* _waitingtime 0.5))
    (bind _asbp_top_down_character (Utilities|Casting|CastToBP_TopDownCharacter (Game|GetPlayerCharacter 0))
      (:then
        (Game|Player|SetViewTargetwithBlend (Game|GetPlayerController 0) _asbp_top_down_character _blend_time "VTBlend_Linear" 0.0 false)
        (Utilities|FlowControl|Delay _blend_time)
        (Actor|DestroyActor)
        (Input|EnableInput (Game|Player|GetPlayerPawn 0) (Game|GetPlayerController 0)))
      (:CastFailed
        (Development|PrintString "Error on the Player casting")))))

(event EventBeginPlay
  (for _array_element (Variables|Keys|GetKeysNeeded)
    (EventDispatchers|BindEventtoOnKeyPicked _array_element (delegate Custom|EmptyKeysNeeded))))

(fn ConstructionScript)