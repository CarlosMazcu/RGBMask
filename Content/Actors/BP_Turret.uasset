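; BP_Turret is a turret that automatically fires pooled BP_Projectiles along its mesh's forward vector.
; A Delay on Tick paces shots by FireRate, then acquires a projectile from ProjectilPool with a spawn transform, velocity and lifetime.
; Each shot receives its pool owner and initial speed, is set hidden in the hardcoded Blue mask, and gets the matching colour material.
; The player-cast and direct SpawnActor paths are unused.
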(event EventBeginPlay)

(event Collision|EventActorBeginOverlap
  (params (OtherActor :type Actor%20Object%20Reference)))

(event EventTick
  (params (DeltaSeconds :type Float%20%28single-precision%29))
  (bind _array (Utilities|Array|MakeArray "Blue"))
  (Utilities|FlowControl|Delay (Variables|Default|GetFireRate))
  (bind _returnvalue (Class|ProjectilPoolComponent|AcquireProjectile (Variables|Default|GetProjectilPool) (Utilities|Struct|MakeProjectileSpawnParams (Transformation|GetWorldTransform (Variables|Default|GetScene)) (* (Variables|Default|GetProjectileSpeed) (Math|Vector|GetForwardVector (Variables|Default|GetStaticMesh))) 6.0)))
  (bind _asbp_projectile (Utilities|Casting|CastToBP_Projectile _returnvalue))
  (Variables|/Game/Actors/BP_Projectile.BP_Projectile_C|SetPoolOwner _asbp_projectile (Variables|Default|GetProjectilPool))
  (Variables|/Script/Engine.ProjectileMovementComponent|SetInitialSpeed (Variables|/Game/Actors/BP_Projectile.BP_Projectile_C|GetProjectileMovement _asbp_projectile) (Variables|Default|GetProjectileSpeed))
  (Class|MaskVisibilityComponent|SetHiddeninMask (Variables|/Game/Actors/BP_Projectile.BP_Projectile_C|GetMaskVisibility _asbp_projectile) _array)
  (switch Utilities|FlowControl|Switch|SwitchonEMaskType (Utilities|Array|Get(acopy) _array)
    (:Red
      (Rendering|Material|SetMaterial (Variables|/Game/Actors/BP_Projectile.BP_Projectile_C|GetStaticMesh _asbp_projectile) 0 "/Game/LevelPrototyping/Materials/M_Test_Red.M_Test_Red"))
    (:Green
      (Rendering|Material|SetMaterial (Variables|/Game/Actors/BP_Projectile.BP_Projectile_C|GetStaticMesh _asbp_projectile) 0 "/Game/LevelPrototyping/Materials/M_Test_Green.M_Test_Green"))
    (:Blue
      (Rendering|Material|SetMaterial (Variables|/Game/Actors/BP_Projectile.BP_Projectile_C|GetStaticMesh _asbp_projectile) 0 "/Game/LevelPrototyping/Materials/M_Test_Blue.M_Test_Blue"))
    (:None
      (Rendering|Material|SetMaterial (Variables|/Game/Actors/BP_Projectile.BP_Projectile_C|GetStaticMesh _asbp_projectile) 0 "/Game/LevelPrototyping/Materials/MI_PrototypeGrid_Gray.MI_PrototypeGrid_Gray"))))

(fn ConstructionScript)